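; First-person character Blueprint using Enhanced Input, with throttle-based movement and a camera that looks independently of the body.
; Move input raises a clamped throttle by a set step and captures camera forward as heading, which Tick turns directly into CharacterMovement velocity.
; Look rotates only the camera, Turn yaws the controller, and Jump and Sprint use standard character movement.
; Standard movement, strafe and continuous-throttle variants remain as unconnected nodes.
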(event `self.ReceiveBeginPlay`
  (`|ExecutionSequence`
    (:`then_0`
      ;[1 1 1] Set Base Walk Speed
      (set `CharacterMovementComponent.MaxWalkSpeed` (`self.MaxSpeedBase`) (`self.CharacterMovement`)))
    (:`then_1`
      ;[1 1 1] Init Input
      (bind _asplayer_controller (cast `PlayerController` (`self.GetController`))
        (:`then`
          (bind _returnvalue (pcsubsystem `EnhancedInputLocalPlayerSubsystem` _asplayer_controller))
          (`/Engine/EditorBlueprintResources/StandardMacros.IsValid` _returnvalue
            (:`Is Valid`
              (message `EnhancedInputSubsystemInterface.AddMappingContext` _returnvalue "/Game/Input/IM_Base.IM_Base" 0 (struct)))
            (:`Is Not Valid`
              (`KismetSystemLibrary.PrintString` "NOT VALID"))))
        (:`CastFailed`
          (`KismetSystemLibrary.PrintString` "CAST FAILED"))))))

(event `self.ReceiveTick`
  (params (DeltaSeconds :type "Float (single-precision)"))
  ;[1 1 1] Apply Discrete Throttle
  (set `MovementComponent.Velocity` (* DeltaSeconds (`self.Throttle`) (`self.MovementSpeed`) (`self.Heading`)) (`self.CharacterMovement`)))

(event `EnhancedInput|/Game/Input/IA_Look`
  (params (ActionValue :type "Vector2D Structure") (ElapsedSeconds :type "Float (double-precision)") (TriggeredSeconds :type "Float (double-precision)") (InputAction :type "InputAction Object Reference" :default "/Game/Input/IA_Look.IA_Look"))
  (bind _camera (`self.Camera`))
  (:`Triggered`
    ;[1 1 1] Rotate Camera Independent of Body
    (`SceneComponent.K2_AddRelativeRotation` _camera (`KismetMathLibrary.MakeRotator` 0.0 0.0 ActionValue_X) false false)
    (`SceneComponent.K2_AddLocalRotation` _camera (`KismetMathLibrary.MakeRotator` 0.0 ActionValue_Y) false false)
    (`KismetSystemLibrary.PrintString` (`KismetStringLibrary.Conv_VectorToString` (`SceneComponent.GetForwardVector` _camera)) :!enabledstate Disabled)))

(event `EnhancedInput|/Game/Input/IA_Move`
  (params (ActionValue :type "Vector2D Structure") (ElapsedSeconds :type "Float (double-precision)") (TriggeredSeconds :type "Float (double-precision)") (InputAction :type "InputAction Object Reference" :default "/Game/Input/IA_Move.IA_Move"))
  (:`Triggered`
    ;[1 1 1] Discrete Throttle
    (set `self.Heading` (`SceneComponent.GetForwardVector` (`self.Camera`)))
    (bind _output_get (set `self.Throttle` (`KismetMathLibrary.FClamp` (+ (`self.Throttle`) (`self.ThrottleStep`)) 0.0 (`self.MaxSpeedBase`))))
    (`KismetSystemLibrary.PrintString` (`KismetTextLibrary.Conv_TextToString` (`|FormatText` "Throttle: {0}" _output_get)))))

(event `EnhancedInput|/Game/Input/IA_Turn`
  (params (ActionValue :type "Float (double-precision)") (ElapsedSeconds :type "Float (double-precision)") (TriggeredSeconds :type "Float (double-precision)") (InputAction :type "InputAction Object Reference" :default "/Game/Input/IA_Turn.IA_Turn"))
  (:`Triggered`
    (`self.AddControllerYawInput` (* ActionValue 36.0))
    ;[1 1 1] Print Rotation
    (`KismetSystemLibrary.PrintString` (`KismetTextLibrary.Conv_TextToString` (`|FormatText` "Rotation: {0}" (`KismetMathLibrary.DegAcos` (`KismetMathLibrary.Dot_VectorVector` (`self.GetActorForwardVector`) (`KismetMathLibrary.Vector_Forward`))))) :!enabledstate Disabled)))

(event `EnhancedInput|/Game/Input/IA_Jump`
  (params (ActionValue :type Boolean) (ElapsedSeconds :type "Float (double-precision)") (TriggeredSeconds :type "Float (double-precision)") (InputAction :type "InputAction Object Reference" :default "/Game/Input/IA_Jump.IA_Jump"))
  (:`Triggered`
    (`self.Jump`)))

(event `EnhancedInput|/Game/Input/IA_Sprint`
  (params (ActionValue :type Boolean) (ElapsedSeconds :type "Float (double-precision)") (TriggeredSeconds :type "Float (double-precision)") (InputAction :type "InputAction Object Reference" :default "/Game/Input/IA_Sprint.IA_Sprint"))
  (bind _charactermovement (`self.CharacterMovement`))
  (:`Triggered`
    (set `CharacterMovementComponent.MaxWalkSpeed` (`self.MaxSpeedSprint`) _charactermovement))
  (:`Completed`
    (set `CharacterMovementComponent.MaxWalkSpeed` (`self.MaxSpeedBase`) _charactermovement)))

(fn `UserConstructionScript`)