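; Auto-runner character that drives itself along a stored heading using stepped throttle shifts, with free camera look, braking and jump.
; Tick overwrites movement velocity from summed throttle, gain, decaying boost and brake.
; Throttle input targets camera forward, shifting instantly at low speed, otherwise interpolating heading and gain.
; A triggered, aligned shift snaps heading to angular increments, raises throttle and grants boost; debug prints and disconnected movement experiments remain.
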(event `self.ReceiveBeginPlay`
  (`|ExecutionSequence`
    (:`then_0`
      ;[1 1 1] Set Base Walk Speed
      (set `CharacterMovementComponent.MaxWalkSpeed` (`self.ThrottleMax`) (`self.CharacterMovement`)))
    (:`then_1`
      ;[1 1 1] Init Input
      (bind _asplayer_controller (cast `PlayerController` (`self.GetController`))
        (:`then`
          (bind _returnvalue (pcsubsystem `EnhancedInputLocalPlayerSubsystem` _asplayer_controller))
          (`/Engine/EditorBlueprintResources/StandardMacros.IsValid` _returnvalue
            (:`Is Valid`
              (message `EnhancedInputSubsystemInterface.AddMappingContext` _returnvalue "/Game/Input/IM_Base.IM_Base" 0 (struct)))
            (:`Is Not Valid`
              (`KismetSystemLibrary.PrintString` "NOT VALID"))))
        (:`CastFailed`
          (`KismetSystemLibrary.PrintString` "CAST FAILED"))))))

(event `self.ReceiveTick`
  (params (DeltaSeconds :type "Float (single-precision)"))
  (bind _throttle (`self.Throttle`))
  (bind _throttlebrake (`self.ThrottleBrake`))
  (bind _throttlegain (`self.ThrottleGain`))
  (bind _throttleboost (`self.ThrottleBoost`))
  (bind _headingclamp (`self.HeadingClamp`))
  (bind _returnvalue (`KismetMathLibrary.RadiansToDegrees` (`KismetMathLibrary.Vector_HeadingAngle` (`self.TargetHeading`))))
  (bind _returnvalue_2 (`KismetMathLibrary.FMax` (+ _throttlebrake _throttle _throttlegain _throttleboost)))
  (`|ExecutionSequence`
    (:`then_0`
      ;[1 1 1] Apply Discrete Throttle
      (set `MovementComponent.Velocity` (* _returnvalue_2 DeltaSeconds (`self.MovementSpeed`) (`KismetMathLibrary.Normal` (`self.Heading`))) (`self.CharacterMovement`))
      (`KismetSystemLibrary.PrintString` (`KismetTextLibrary.Conv_TextToString` (`|FormatText` "Base {0} Gain {1} Boost {2} Brake {3} Final: {4} " _throttle _throttlegain _throttleboost _throttlebrake _returnvalue_2))))
    (:`then_1`
      ;[1 1 1] Throttle Shift
      (if (and (< (`KismetMathLibrary.Abs` (- (`KismetMathLibrary.RadiansToDegrees` (`KismetMathLibrary.Vector_HeadingAngle` (`self.Heading`))) (`KismetMathLibrary.RadiansToDegrees` (`KismetMathLibrary.Vector_HeadingAngle` (`self.TargetHeading`))))) (`self.ThrottleShiftHeadingThreshold`)) (`self.ThrottleShiftReady`))
        (set `self.Heading` (`KismetMathLibrary.RotateAngleAxis` (`self.TargetHeading`) (- (* _headingclamp (`KismetMathLibrary.Round` (/ _returnvalue _headingclamp))) _returnvalue) (0.0 0.0 1.0)) :!label _label)
        (set `self.Throttle` (`KismetMathLibrary.FClamp` (+ (`self.Throttle`) (`self.ThrottleStep`)) 0.0 (`self.ThrottleMax`)))
        (set `self.StateThrottleShifting` false)
        (set `self.ThrottleShiftReadyViaBrake` false)
        (set `self.ThrottleShiftReady` false)
        (set `self.ThrottleShiftHeadingInterpolationAlpha` 0.0)
        (set `self.ThrottleShiftThrottleInterpolationAlpha` 0.0)
        (set `self.ThrottleGain` 0.0)
        (set `self.ThrottleBoost` (`self.ThrottleBoostValue`))
        (`KismetSystemLibrary.PrintString` "Shifted" true true (struct :`R` 1.0 :`B` 0.924857 :`A` 1.0) (`self.LoggingDuration`))))
    (:`then_2`
      (if (`self.StateThrottleShifting`)
        (`|ExecutionSequence`
          (:`then_0`
            ;[1 1 1] Calculate Throttle Shift Interpolation
            (set `self.ThrottleShiftHeadingInterpolationAlpha` (+ (* DeltaSeconds (`self.ThrottleShiftHeadingInterpolationRate`)) (`self.ThrottleShiftHeadingInterpolationAlpha`))))
          (:`then_1`
            ;[1 1 1] Calculate Throttle Shift Interpolation
            (set `self.ThrottleShiftThrottleInterpolationAlpha` (+ (* DeltaSeconds (`self.ThrottleShiftThrottleInterpolationRate`)) (`self.ThrottleShiftThrottleInterpolationAlpha`))))
          (:`then_2`
            ;[1 1 1] Lerp Heading
            (set `self.Heading` (`KismetMathLibrary.VLerp` (`self.Heading`) (`self.TargetHeading`) (`self.ThrottleShiftHeadingInterpolationAlpha`))))
          (:`then_3`
            ;[1 1 1] Lerp Throttle
            (set `self.ThrottleGain` (`KismetMathLibrary.Lerp` (`self.ThrottleGain`) (`self.ThrottleGainMax`) (`self.ThrottleShiftThrottleInterpolationAlpha`)))))))
    (:`then_3`
      ;[1 1 1] Throttle Boost Decay
      (set `self.ThrottleBoost` (`KismetMathLibrary.Lerp` (`self.ThrottleBoost`) 0.0 (* (`self.ThrottleBoostDecay`) DeltaSeconds))))))

(event `EnhancedInput|/Game/Input/IA_Look`
  (params (ActionValue :type "Vector2D Structure") (ElapsedSeconds :type "Float (double-precision)") (TriggeredSeconds :type "Float (double-precision)") (InputAction :type "InputAction Object Reference" :default "/Game/Input/IA_Look.IA_Look"))
  (bind _camera (`self.Camera`))
  (:`Triggered`
    ;[1 1 1] Rotate Camera Independent of Body
    (`SceneComponent.K2_AddRelativeRotation` _camera (`KismetMathLibrary.MakeRotator` 0.0 0.0 ActionValue_X) false false)
    (`SceneComponent.K2_AddLocalRotation` _camera (`KismetMathLibrary.MakeRotator` 0.0 ActionValue_Y) false false)))

(event `EnhancedInput|/Game/Input/IA_Brake`
  (params (ActionValue :type Boolean) (ElapsedSeconds :type "Float (double-precision)") (TriggeredSeconds :type "Float (double-precision)") (InputAction :type "InputAction Object Reference" :default "/Game/Input/IA_Brake.IA_Brake"))
  (:`Triggered`
    (set `self.ThrottleBrake` (`KismetMathLibrary.Lerp` (`self.ThrottleBrake`) (* (`self.Throttle`) (`self.ThrottleBrakeMax`) -1.0) (* (`self.ThrottleBrakeDeceleration`) (stale `self.ReceiveTick` DeltaSeconds)))))
  (:`Completed`
    (set `self.ThrottleBrake` 0.0)))

(event `EnhancedInput|/Game/Input/IA_Throttle`
  (params (ActionValue :type Boolean) (ElapsedSeconds :type "Float (double-precision)") (TriggeredSeconds :type "Float (double-precision)") (InputAction :type "InputAction Object Reference" :default "/Game/Input/IA_Throttle.IA_Throttle"))
  (bind _loggingduration (`self.LoggingDuration`))
  (bind _loggingduration_2 (`self.LoggingDuration`))
  (:`Triggered`
    (set `self.ThrottleShiftReady` true)
    (`KismetSystemLibrary.PrintString` "Ready" true true (struct :`R` 1.0 :`G` 0.463901 :`A` 1.0) _loggingduration_2)
    (`|ExecutionSequence` :!label _label_2
      (:`then_0`
        (`KismetSystemLibrary.PrintString` (`KismetTextLibrary.Conv_TextToString` (`|FormatText` "Velocity {0}" (`self.Throttle`))) true true (struct :`G` 0.66 :`B` 1.0 :`A` 1.0) _loggingduration))
      (:`then_1`
        (`KismetSystemLibrary.PrintString` (`KismetTextLibrary.Conv_TextToString` (`|FormatText` "Heading {0}" (`KismetMathLibrary.Vector_HeadingAngle` (`self.Heading`)))) true true (struct :`G` 0.66 :`B` 1.0 :`A` 1.0) _loggingduration))
      (:`then_2`
        (`KismetSystemLibrary.PrintString` (`KismetTextLibrary.Conv_TextToString` (`|FormatText` "Target Heading {0}" (`KismetMathLibrary.Vector_HeadingAngle` (`self.TargetHeading`)))) true true (struct :`G` 0.66 :`B` 1.0 :`A` 1.0) _loggingduration)
        (`KismetSystemLibrary.PrintString` (`KismetTextLibrary.Conv_TextToString` (`|FormatText` "To Target Heading {0}" (`KismetMathLibrary.Abs` (- (`KismetMathLibrary.RadiansToDegrees` (`KismetMathLibrary.Vector_HeadingAngle` (`self.Heading`))) (`KismetMathLibrary.RadiansToDegrees` (`KismetMathLibrary.Vector_HeadingAngle` (`self.TargetHeading`))))))) true true (struct :`G` 0.66 :`B` 1.0 :`A` 1.0) _loggingduration))))
  (:`Started`
    (if (< (`KismetMathLibrary.VSize` (`self.GetVelocity`)) 350.0)
      (`|ExecutionSequence`
        (:`then_0`
          _)
        (:`then_1`
          (goto _label)))
      (else
        ;[1 1 1] Begin Throttle Interpolation
        (set `self.StateThrottleShifting` true)))
    (set `self.TargetHeading` (`SceneComponent.GetForwardVector` (`self.Camera`)))
    (`KismetSystemLibrary.PrintString` "Begin" true true (struct :`G` 1.0 :`B` 0.440684 :`A` 1.0) _loggingduration_2)
    (goto _label_2))
  (:`Canceled`
    (set `self.StateThrottleShifting` false)
    (`KismetSystemLibrary.PrintString` "Canceled" true true (struct :`R` 1.0 :`G` 0.046263 :`A` 1.0) _loggingduration_2)
    (goto _label_2)))

(event `EnhancedInput|/Game/Input/IA_Brake`
  (params (ActionValue :type Boolean) (ElapsedSeconds :type "Float (double-precision)") (TriggeredSeconds :type "Float (double-precision)") (InputAction :type "InputAction Object Reference" :default "/Game/Input/IA_Brake.IA_Brake")))

(event `EnhancedInput|/Game/Input/IA_Move`
  (params (ActionValue :type "Vector2D Structure") (ElapsedSeconds :type "Float (double-precision)") (TriggeredSeconds :type "Float (double-precision)") (InputAction :type "InputAction Object Reference" :default "/Game/Input/IA_Move.IA_Move")))

(event `EnhancedInput|/Game/Input/IA_Turn`
  (params (ActionValue :type "Float (double-precision)") (ElapsedSeconds :type "Float (double-precision)") (TriggeredSeconds :type "Float (double-precision)") (InputAction :type "InputAction Object Reference" :default "/Game/Input/IA_Turn.IA_Turn")))

(event `EnhancedInput|/Game/Input/IA_Jump`
  (params (ActionValue :type Boolean) (ElapsedSeconds :type "Float (double-precision)") (TriggeredSeconds :type "Float (double-precision)") (InputAction :type "InputAction Object Reference" :default "/Game/Input/IA_Jump.IA_Jump"))
  (:`Triggered`
    (`self.Jump`)))

(fn `UserConstructionScript`)